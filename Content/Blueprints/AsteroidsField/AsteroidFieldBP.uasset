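; Asteroid field actor that scatters big and small asteroids at random inside a spherical radius.
; The construction script adds both size groups as hierarchical instanced static mesh instances, with counts set by variables and no active event logic.
; Each instance gets a random direction, distance, rotation and non-uniform scale.
; Randomness is unseeded, and linear distance sampling clusters asteroids toward the center.
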(fn `UserConstructionScript`
  (`|ExecutionSequence`
    (:`then_0`
      (for _ (range 1 (+ (`self.NumBigAsteroids`) 1))
        (`InstancedStaticMeshComponent.AddInstance` (`self.HierarchicalInstancedStaticMesh`) (`KismetMathLibrary.MakeTransform` (* (`KismetMathLibrary.RandomUnitVector`) (`KismetMathLibrary.RandomFloatInRange` 0.0 (`self.FieldRadius`))) (`KismetMathLibrary.RandomRotator` true) (+ (* (`KismetMathLibrary.RandomUnitVector`) 20.0) 20.0)))))
    (:`then_1`
      (for _ (range 1 (+ (`self.NumSmallAsteroids`) 1))
        (`InstancedStaticMeshComponent.AddInstance` (`self.HierarchicalInstancedStaticMesh`) (`KismetMathLibrary.MakeTransform` (* (`KismetMathLibrary.RandomUnitVector`) (`KismetMathLibrary.RandomFloatInRange` 0.0 (`self.FieldRadius`))) (`KismetMathLibrary.RandomRotator` true) (+ (* (`KismetMathLibrary.RandomUnitVector`) 0.5) 1.0)))))))