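; FalconHUDBP creates and controls the on-screen Falcon HUD widget.
; On BeginPlay it creates a TemplateFalconHUDWidget for the first player controller, adds it to the viewport and starts it collapsed.
; A SetFalconHUDVisibility event switches the widget between hit-test invisible when shown and collapsed when hidden.
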(event `self.ReceiveBeginPlay`
  (bind _returnvalue (`|CreateWidget` (`self.templateFalconHUDWidget`) (`GameplayStatics.GetPlayerController` 0)))
  (bind _output_get (set `self.FalconHudWidget` _returnvalue))
  (`UserWidget.AddToViewport` _output_get 0)
  (`Widget.SetVisibility` (`self.FalconHudWidget`) "Collapsed"))

(event `self.SetFalconHUDVisibility`
  (params (IsVisible :type Boolean))
  (bind _falconhudwidget (`self.FalconHudWidget`))
  (if IsVisible
    (`Widget.SetVisibility` _falconhudwidget "HitTestInvisible")
    (else
      (`Widget.SetVisibility` _falconhudwidget "Collapsed"))))

(fn `UserConstructionScript`)